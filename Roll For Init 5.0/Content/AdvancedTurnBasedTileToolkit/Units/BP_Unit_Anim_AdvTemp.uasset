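; Turn-based toolkit unit Blueprint that shows and clears a floating damage popup in response to animation actions.
; AnimateAction waits the action's activation delay, then matches its name to display the first string as a red negative value or blank the text.
; TurnOnOffPopup sets the DamagePopup text and color, then rotates it once to face the BP_GridCamera camera.
; ModifyHealth only forwards to the parent.
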(event Custom|TurnOnOffPopup
  (params (Text%20String :type String) (Text%20Color :type Color%20Structure))
  (Rendering|Components|TextRender|SetText (Variables|Default|GetDamagePopup) (Utilities|Text|ToText(String) Text%20String))
  (Rendering|Components|TextRender|SetTextRenderColor (Variables|Default|GetDamagePopup) Text%20Color)
  (bind _outactors (Actor|GetAllActorsOfClass "/Game/AdvancedTurnBasedTileToolkit/Core/BP_GridCamera.BP_GridCamera_C"))
  (for _array_element _outactors
    (Transformation|SetWorldRotation (Variables|Default|GetDamagePopup) (Math|Rotator|FindLookatRotation (Transformation|GetWorldLocation (Variables|Default|GetDamagePopup)) (Transformation|GetWorldLocation (Variables|/Game/AdvancedTurnBasedTileToolkit/Core/BP_GridCamera.BP_GridCamera_C|GetCamera _array_element))) false false)))

(event Custom|AnimateAction_1
  (params (CallingActionManager :type BP%20Action%20Manager%20Object%20Reference) (Action :type F%20Action%20Structure))
  (bind (_executingobject _actionname _binstantdeactivate _atcustomindex _bwithprevious _activationdelay _booleans _integers _floats _strings) (Utilities|Struct|BreakFAction Action))
  (bind _returnvalue (Math|Color|MakeColor 1.0 0.0 0.0))
  (bind _returnvalue_2 (Math|Conversions|ToColor(LinearColor) _returnvalue))
  (Utilities|FlowControl|Delay _activationdelay)
  (switch name _actionname
    (:TurnOffPopUp
      (CallFunction|TurnonOffPopup (Utilities|String|MakeLiteralString " ") _returnvalue_2))
    (:TurnOnPopup
      (CallFunction|TurnonOffPopup (Utilities|String|Append "-" (Utilities|Array|Get(acopy) _strings)) _returnvalue_2))))

(event EventBeginPlay
  (|CallParentFunction) ; This node is disabled and will not be called.\nDrag off pins to build functionality.
)

(event Collision|EventActorBeginOverlap
  (params (OtherActor :type Actor%20Object%20Reference)))

(event EventTick
  (params (DeltaSeconds :type Float%20%28single-precision%29)))

(event EventModifyHealth
  (params (Change :type Float%20%28single-precision%29) (bAutoAnimate :type Boolean) (EndDelay :type Float%20%28single-precision%29) (Damage :type Float%20%28single-precision%29))
  (|CallParentFunction 0.0 bAutoAnimate -1.0 Damage))

(fn ConstructionScript
  (|CallParentFunction))